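; Player info for a Pavlov admin-menu mod, handling admin actions: kick, kill one or all, change skin, teleport to admin, end match.
; Actions find players by SteamId or name, then call their Admin_PlayerInfo or Admin_PlayerProxy, or Admin_GameLogic for match end.
; ServerSpawnMenu runs a ModList/debug-name check, currently fed empty strings, before ClientMenu attaches menu and widget interactor to off and dominant hands.
; LoadAllNames refreshes the menu's player list.
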(event Custom|Kill%20Player%20Server
  (params (Name :type String))
  ;[1 1 1] Kill Player
  (bind _asadmin_game_logic (Utilities|Casting|CastToAdmin_GameLogic (Class|PavlovLibrary|GetGameLogic)))
  (for _array_element (Default|GetPlayers _asadmin_game_logic)
    (bind _returnvalue (CallFunction|IsforPcCheckNameChange _array_element))
    (if (Utilities|Enum|Equal(Enum) _returnvalue Name)
      (bind _playerstatus (Class|PavlovProxyStatics|GetPavlovPlayerStatus _array_element))
      (bind _asadmin_player_proxy (Utilities|Casting|CastToAdmin_PlayerProxy (Class|PavlovLibrary|GetPlayerProxy (.pawn _playerstatus))))
      (Default|KillPlayer _asadmin_player_proxy true))))

(event Custom|Teleport%20Player%20To%20Admin
  (params (Player%20Name :type String) (Admin :type Actor%20Object%20Reference))
  ;[1 1 1] Teleport Player To Admin
  (bind _asadmin_game_logic (Utilities|Casting|CastToAdmin_GameLogic (Class|PavlovLibrary|GetGameLogic)))
  (for _array_element (Default|GetPlayers _asadmin_game_logic)
    (bind _returnvalue (CallFunction|IsforPcCheckNameChange _array_element))
    (if (Utilities|Enum|Equal(Enum) _returnvalue Player%20Name)
      (bind _playerstatus (Class|PavlovProxyStatics|GetPavlovPlayerStatus _array_element))
      (bind _asadmin_player_proxy (Utilities|Casting|CastToAdmin_PlayerProxy (Class|PavlovLibrary|GetPlayerProxy (.pawn _playerstatus))))
      (Default|ServerTeleportPlayer _asadmin_player_proxy Admin))))

(event Custom|Kick%20Player
  (params (Name :type String))
  ;[1 1 1] Kick Player
  (bind _asadmin_game_logic (Utilities|Casting|CastToAdmin_GameLogic (Class|PavlovLibrary|GetGameLogic)))
  (for _array_element (Default|GetPlayers _asadmin_game_logic)
    (bind _returnvalue (CallFunction|IsforPcCheckNameChange _array_element))
    (if (Utilities|Enum|Equal(Enum) _returnvalue Name)
      (bind _asadmin_player_info (Utilities|Casting|CastToAdmin_PlayerInfo (Class|PavlovLibrary|GetPlayerInfo _array_element)))
      (CallFunction|ServerKick _asadmin_player_info))))

(event Custom|Server%20Kick
  ;[1 1 1] Kick Player
  (CallFunction|ClientKick))

(event Custom|Client%20Kick
  ;[1 1 1] Kick Player
  (Development|ExecuteConsoleCommand "disconnect" 0))

(event Custom|Kill%20All%20Player%20Server%20PlPr
  ;[1 1 1] Kill All Players
  (bind _asadmin_game_logic (Utilities|Casting|CastToAdmin_GameLogic (Class|PavlovLibrary|GetGameLogic)))
  (for _array_element (Default|GetPlayers _asadmin_game_logic)
    (bind _playerstatus (Class|PavlovProxyStatics|GetPavlovPlayerStatus _array_element))
    (bind _asadmin_player_proxy (Utilities|Casting|CastToAdmin_PlayerProxy (Class|PavlovLibrary|GetPlayerProxy (.pawn _playerstatus))))
    (Default|KillPlayer _asadmin_player_proxy true)))

(event Custom|Load%20All%20Names
  ;[1 1 1] Load Names
  (Variables|AdminMenu|SetAll%20Names (Utilities|Array|MakeArray))
  (bind _asadmin_game_logic (Utilities|Casting|CastToAdmin_GameLogic (Class|PavlovLibrary|GetGameLogic)))
  (for _array_element (Default|GetPlayers _asadmin_game_logic)
    (bind _returnvalue (CallFunction|IsforPcCheckNameChange _array_element))
    (Utilities|Array|Add (Variables|AdminMenu|GetAll%20Names) _returnvalue))
  (CallFunction|ClientLoadNames))

(event Custom|Client%20Load%20Names
  ;[1 1 1] Load Names
  (bind _asadmin_menu_widget (Utilities|Casting|CastToAdmin_Menu_Widget (UserInterface|GetUserWidgetObject (Variables|/Game/CustomMaps/AdminMenu/Envy/Blueprints/WorldDeathMenu.WorldDeathMenu_C|GetWidget (Variables|AdminMenu|GetAdminMenu)))))
  (Default|LoadedNames _asadmin_menu_widget))

(event Custom|Server%20Spawn%20Menu
  ;[1 1 1] Spawn Mod Menu
  (bind _player_valid (CallFunction|MenuCheck))
  (if _player_valid
    (CallFunction|ClientMenu)))

(event Custom|Client%20Menu
  ;[1 1 1] Spawn Mod Menu
  (bind (_mainhand _offhand _successful _pawn) (CallFunction|GetHands (Variables|AdminMenu|GetRight%20Hand%20Dominant)))
  (bind _returnvalue (Game|SpawnActorfromClass "/Game/CustomMaps/AdminMenu/Envy/AdminMenu/WidgetInteractor.WidgetInteractor_C" (Transformation|GetWorldTransform _mainhand) "Undefined" _pawn 0))
  (bind _output_get (Variables|AdminMenu|SetWidget%20Ineractor _returnvalue))
  (Transformation|AttachComponentToComponent _output_get _mainhand "None" "SnapToTarget" "SnapToTarget" "KeepWorld" true)
  (bind _returnvalue_2 (Game|SpawnActorfromClass "/Game/CustomMaps/AdminMenu/Envy/Blueprints/WorldDeathMenu.WorldDeathMenu_C" (Transformation|GetWorldTransform _offhand) "Undefined" _pawn 0))
  (bind _output_get_2 (Variables|AdminMenu|SetAdminMenu _returnvalue_2))
  (Transformation|AttachComponentToComponent _output_get_2 _offhand "None" "SnapToTarget" "SnapToTarget" "KeepWorld" true))

(event Custom|Mark%20Dominant
  (params (Right%20Hand%20Dominant :type Boolean))
  ;[1 1 1] Mark Dominant
  (Variables|AdminMenu|SetRight%20Hand%20Dominant Right%20Hand%20Dominant))

(event Custom|End%20Match
  ;[1 1 1] End Match
  (bind _asadmin_game_logic (Utilities|Casting|CastToAdmin_GameLogic (Class|PavlovLibrary|GetGameLogic)))
  (Class|PavlovGameLogic|SetRoundState _asadmin_game_logic "Ended"))

(event Custom|Change%20Player%20Skin
  (params (Name :type String) (Skin :type Name))
  ;[1 1 1] Change PLayer Skin
  (bind _asadmin_game_logic (Utilities|Casting|CastToAdmin_GameLogic (Class|PavlovLibrary|GetGameLogic)))
  (for _array_element (Default|GetPlayers _asadmin_game_logic)
    (bind _returnvalue (CallFunction|IsforPcCheckNameChange _array_element))
    (if (Utilities|Enum|Equal(Enum) _returnvalue Name)
      (bind _playerstatus (Class|PavlovProxyStatics|GetPavlovPlayerStatus _array_element))
      (bind _asadmin_player_proxy (Utilities|Casting|CastToAdmin_PlayerProxy (Class|PavlovLibrary|GetPlayerProxy (.pawn _playerstatus))))
      (Default|SetPlayerSkin _asadmin_player_proxy Skin))))

(fn GetHands
  (params (Right%20Hand%20Dominant :type Boolean))
  (bind _playerstatus (Class|PavlovProxyStatics|GetPavlovPlayerStatus (Class|PavlovPlayerInfo|GetPlayerState)))
  (for _array_element (Components|GetChildrenComponents (Variables|/Script/Engine.Actor|GetRootComponent (.Pawn (Utilities|Struct|BreakPavlovPlayerStatus _playerstatus))) true)
    (bind _asmotion_controller_component (Utilities|Casting|CastToMotionControllerComponent _array_element))
    (switch name (Variables|/Script/HeadMountedDisplay.MotionControllerComponent|GetMotionSource _asmotion_controller_component)
      (:Left
        (LocalVariables|SetLeft%20Hand _asmotion_controller_component))
      (:Right
        (LocalVariables|SetRight%20Hand _asmotion_controller_component))))
  (return (select Right%20Hand%20Dominant (LocalVariables|GetRight%20Hand) (LocalVariables|GetLeft%20Hand)) (select Right%20Hand%20Dominant (LocalVariables|GetLeft%20Hand) (LocalVariables|GetRight%20Hand)) (Utilities|IsBothValid (LocalVariables|GetLeft%20Hand) (LocalVariables|GetRight%20Hand)) (.Pawn (Utilities|Struct|BreakPavlovPlayerStatus _playerstatus))))

(fn MenuCheck
  (Development|PrintString "********Running Menu Check For Admins To Spawn Menu**********" true true "(R=0.000000,G=0.660000,B=1.000000,A=1.000000)" 5.0)
  (Class|PavlovProxyStatics|GetPavlovPlayerStatus (Class|PavlovPlayerInfo|GetPlayerState))
  (bind _asadmin_game_logic (Utilities|Casting|CastToAdmin_GameLogic (Class|PavlovLibrary|GetGameLogic)))
  (Development|PrintString (select (or (Utilities|Array|ContainsItem (Variables|/Game/CustomMaps/AdminMenu/Envy/Blueprints/Admin_GameLogic.Admin_GameLogic_C|GetMod%20List _asadmin_game_logic) "") (Utilities|Enum|Equal(Enum) "" (Variables|Debugging|GetEnterMapMakerNameHereFor%20Debugging%20Purposes))) (Utilities|String|Append "<<<<<<Player Name " "" "   YYYEEESSS Listed As Admin>>>>") "<<<Player Name Not Listed As Admin>>>>>"))
  (return (or (Utilities|Array|ContainsItem (Variables|/Game/CustomMaps/AdminMenu/Envy/Blueprints/Admin_GameLogic.Admin_GameLogic_C|GetMod%20List _asadmin_game_logic) "") (Utilities|Enum|Equal(Enum) "" (Variables|Debugging|GetEnterMapMakerNameHereFor%20Debugging%20Purposes)))))

(fn IsforPcCheckNameChange
  (params (PlayerState :type Player%20State%20Object%20Reference))
  (bind _playerstatus (Class|PavlovProxyStatics|GetPavlovPlayerStatus PlayerState))
  (return (select (Variables|Default|GetIs%20For%20PC?) (.SteamId (Utilities|Struct|BreakPavlovPlayerStatus _playerstatus)) (Variables|/Script/Engine.PlayerState|GetPlayerName PlayerState))))