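; Blueprint function library of Pavlov helper utilities in the Envy AdminMenu custom map folder.
; IsPavPawn identifies Pavlov pawns by matching "Pawn" at a fixed position in the display name, avoiding a class cast.
; GetHands searches the pawn root's child components for left and right MotionControllerComponents, returning both with a success flag.
; ManageTags adds or removes a unique tag on a valid PlayerState.
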(fn IsPavPawn?
  (params (Pawn :type Pawn%20Object%20Reference))
  (return (Utilities|Enum|Equal(Enum) (Utilities|String|GetSubstring (Utilities|GetDisplayName Pawn) 9 4) "Pawn")))

(fn GetHands
  (params (Pawn :type Pawn%20Object%20Reference))
  (Utilities|IsValid Pawn
    (:Is%20Valid
      (bind _array_element (Utilities|Array|ForEachLoopwithBreak (Components|GetChildrenComponents (Variables|/Script/Engine.Actor|GetRootComponent Pawn) true) :!label _label)
        (:LoopBody
          (bind _asmotion_controller_component (Utilities|Casting|CastToMotionControllerComponent _array_element))
          (switch name (Variables|/Script/HeadMountedDisplay.MotionControllerComponent|GetMotionSource _asmotion_controller_component)
            (:Left
              (LocalVariables|SetL_HandL _asmotion_controller_component)
              (Utilities|IsValid (LocalVariables|GetL_HandR)
                (:Is%20Valid
                  (LocalVariables|SetL_Successful true)
                  (goto _label Break))))
            (:Right
              (LocalVariables|SetL_HandR _asmotion_controller_component)
              (Utilities|IsValid (LocalVariables|GetL_HandL)
                (:Is%20Valid
                  (LocalVariables|SetL_Successful true)
                  (goto _label Break))))))
        (:Completed
          (return (LocalVariables|GetL_Successful) (LocalVariables|GetL_HandL) (LocalVariables|GetL_HandR)))))
    (:Is%20Not%20Valid
      (return false 0 0))))

(fn ManageTags
  (params (PlayerState :type Player%20State%20Object%20Reference) (AddTag? :type Boolean) (Tag :type Name))
  (LocalVariables|GetPlayerState
    (:then
      (if AddTag?
        (Utilities|Array|AddUnique (Variables|/Script/Engine.Actor|GetTags PlayerState) Tag)
        (else
          (Utilities|Array|RemoveItem (Variables|/Script/Engine.Actor|GetTags PlayerState) Tag)))
      (return))
    (:else
      (return))))