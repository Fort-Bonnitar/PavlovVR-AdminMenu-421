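; Per-player Pavlov VR proxy for an admin menu mod, spawning the hand-attached menu and handling admin actions on its pawn.
; After a delayed BeginPlay, ModList names get the Admin skin and damage immunity, but both branches spawn the menu spawner and widget interactor.
; Admin_PlayerInfo records the dominant hand and spawns the UI.
; Server/Client event pairs and other events handle kill, kick, teleport, walk speed, skin toggling and name lists.
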(event Custom|Sets%20Player%20Skin%20Invisible
  ;[1 1 1] Sets Player Invisible
  (Utilities|FlowControl|FlipFlop
    (:A
      (Networking|SwitchHasAuthority
        (:Authority
          (Class|PavlovPlayerProxy|SetPlayerSkin "Admin"))))
    (:B
      (Networking|SwitchHasAuthority
        (:Authority
          (Class|PavlovPlayerProxy|SetPlayerSkin "nato"))))))

(event Custom|Kill%20all%20Players%20Server
  ;[1 1 1] Kill All Players
  (Game|Damage|ApplyDamage (Class|PavlovPlayerProxy|GetPawn) 3e+03 0 0))

(event Custom|Set%20Player%20Skin
  (params (Skin :type Name))
  ;[1 1 1] Set Player Skin
  (Networking|SwitchHasAuthority
    (:Authority
      (Class|PavlovPlayerProxy|SetPlayerSkin Skin))))

(event Custom|Kill%20Player
  (params (Remove%20Body :type Boolean))
  ;[1 1 1] Kill Player
  (Variables|Gameplay|SetRemove%20Body Remove%20Body)
  (Game|Damage|ApplyDamage (Class|PavlovPlayerProxy|GetPawn) 3e+03 0 0))

(event Custom|Trigger%20Spawn%20UI
  ;[1 1 1] Spawn UI
  (CallFunction|SpawnUI))

(event Custom|Load%20All%20Names
  ;[1 1 1] Load Names
  (Utilities|Array|Clear (Variables|Gameplay|GetAll%20Names))
  (bind _asadmin_game_logic (Utilities|Casting|CastToAdmin_GameLogic (Class|PavlovLibrary|GetGameLogic)))
  (for _array_element (Default|GetPlayers _asadmin_game_logic)
    (Utilities|Array|Add (Variables|Gameplay|GetAll%20Names) (Variables|/Script/Engine.PlayerState|GetPlayerName _array_element))))

(event Custom|Teleport%20Player
  (params (Admin :type Actor%20Object%20Reference))
  ;[1 1 1] Teleport Player
  (Transformation|SetActorTransform (Class|PavlovPlayerProxy|GetPawn) (Transformation|GetActorTransform Admin)))

(event Custom|Server%20Teleport%20Player
  (params (Admin :type Actor%20Object%20Reference))
  ;[1 1 1] Teleport Player
  (CallFunction|TeleportPlayer Admin))

(event Custom|Spawn%20UI
  (bind _returnvalue (Class|PavlovPlayerProxy|GetPawn))
  ;[1 1 1] Spawn UI
  (Utilities|FlowControl|Delay 1.0)
  (bind _right_hand (CallFunction|GetHands _returnvalue))
  (bind _asadmin_player_info (Utilities|Casting|CastToAdmin_PlayerInfo (Class|PavlovLibrary|GetPlayerInfo (Variables|/Script/Engine.Pawn|GetPlayerState _returnvalue)))
    (:then
      (Default|MarkDominant _asadmin_player_info (== _right_hand (Transformation|GetAttachParent (Transformation|GetAttachParent (Transformation|GetAttachParent (.dominanthand (Variables|Default|GetHandsProxy)))))))
      (Variables|Default|SetPlayer%20Info _asadmin_player_info)
      (Default|ServerSpawnMenu _asadmin_player_info))
    (:CastFailed
      (Development|PrintString "Cast To Player Info Inside the Player Proxy Failed!!!!!" true true "(R=1.000000,G=0.000000,B=0.005922,A=1.000000)" 3e+01))))

(event Custom|Set%20Walk%20Speed
  (params (Slow :type Boolean))
  ;[1 1 1] Set Walk Speed
  (bind _ascharacter (Utilities|Casting|CastToCharacter (Class|PavlovPlayerProxy|GetPawn)))
  (Variables|/Script/Engine.CharacterMovementComponent|SetMaxWalkSpeed (Variables|/Script/Engine.Character|GetCharacterMovement _ascharacter) (Math|Float|SelectFloat 1.8e+02 3e+02 Slow)))

(event Custom|Server%20Kick
  ;[1 1 1] Kick Player
  (CallFunction|ClientKick))

(event Custom|Client%20Kick
  ;[1 1 1] Kick Player
  (Development|ExecuteConsoleCommand "disconnect" 0))

(event Custom|Server%20Mark%20Dominant
  (bind _returnvalue (Class|PavlovPlayerProxy|GetPawn))
  ;[1 1 1] Mark Dominant Hand
  (bind _right_hand (CallFunction|GetHands _returnvalue))
  (bind _asadmin_player_info (Utilities|Casting|CastToAdmin_PlayerInfo (Class|PavlovLibrary|GetPlayerInfo (Variables|/Script/Engine.Pawn|GetPlayerState _returnvalue)))
    (:then
      (Default|MarkDominant _asadmin_player_info (== _right_hand (Transformation|GetAttachParent (Transformation|GetAttachParent (Transformation|GetAttachParent (.dominanthand (Variables|Default|GetHandsProxy)))))))
      (Variables|Default|SetPlayer%20Info _asadmin_player_info)
      (CallFunction|TriggerSpawnUI))
    (:CastFailed
      (Development|PrintString "Cast To Player Info Inside the Player Proxy Failed!!!!!" true true "(R=1.000000,G=0.000000,B=0.005922,A=1.000000)" 3e+01))))

(event Custom|Load%20Names
  ;[1 1 1] Load Names
  (Utilities|Array|Clear (Variables|Core|GetAlive%20Players))
  (Utilities|Array|Clear (Variables|Gameplay|GetName%20Array))
  (bind _asadmin_game_logic (Utilities|Casting|CastToAdmin_GameLogic (Class|PavlovLibrary|GetGameLogic)))
  (for _array_element (select (Variables|/Game/CustomMaps/AdminMenu/Envy/Blueprints/Admin_GameLogic.Admin_GameLogic_C|GetDebug%20Build _asadmin_game_logic) (Default|GetPlayers _asadmin_game_logic) (Variables|/Game/CustomMaps/AdminMenu/Envy/Blueprints/Admin_GameLogic.Admin_GameLogic_C|GetCurrent%20Players _asadmin_game_logic))
    (bind _playerstatus (Class|PavlovProxyStatics|GetPavlovPlayerStatus _array_element))
    (if (not (.bdead _playerstatus))
      (Utilities|Array|AddUnique (Variables|Core|GetAlive%20Players) (.playerstate _playerstatus))
      (Utilities|Array|AddUnique (Variables|Gameplay|GetName%20Array) (Variables|/Script/Engine.PlayerState|GetPlayerName (.playerstate _playerstatus))))))

(event Custom|Spawn%20My%20Admin%20Server
  ;[1 1 1] Replicated Admin Menu Spawn
  (CallFunction|SpawnMyAdminClient))

(event Custom|Spawn%20My%20Admin%20Client
  (bind _returnvalue (Class|PavlovPlayerProxy|GetPawn))
  (bind _handsproxy (Variables|Default|GetHandsProxy))
  (bind _returnvalue_2 (Transformation|GetAttachParent (.nondominanthand _handsproxy)))
  (bind _returnvalue_3 (Transformation|GetAttachParent (.dominanthand _handsproxy)))
  (bind _returnvalue_4 (Transformation|GetAttachParent _returnvalue_2))
  (bind _returnvalue_5 (Transformation|GetAttachParent _returnvalue_3))
  (bind _returnvalue_6 (Transformation|GetAttachParent _returnvalue_4))
  (bind _returnvalue_7 (Transformation|GetAttachParent _returnvalue_5))
  ;[1 1 1] Replicated Admin Menu Spawn
  (CallFunction|ServerMarkDominant)
  (bind _returnvalue_8 (Game|SpawnActorfromClass "/Game/CustomMaps/AdminMenu/Envy/AdminMenu/MyAdminSpawner.MyAdminSpawner_C" (Transformation|GetWorldTransform _returnvalue_6) "Undefined" _returnvalue 0))
  (Transformation|AttachComponentToComponent _returnvalue_8 _returnvalue_6 "None" "SnapToTarget" "SnapToTarget" "KeepWorld" true)
  (bind _returnvalue_9 (Game|SpawnActorfromClass "/Game/CustomMaps/AdminMenu/Envy/AdminMenu/WidgetInteractor.WidgetInteractor_C" (Transformation|GetWorldTransform _returnvalue_7) "Undefined" _returnvalue 0))
  (bind _output_get (Variables|Gameplay|SetWidgetInteractor _returnvalue_9))
  (Transformation|AttachComponentToComponent _output_get _returnvalue_7 "None" "SnapToTarget" "SnapToTarget" "KeepWorld" true))

(event EventBeginPlay
  ;[1 1 1] Begin Play
  (Utilities|FlowControl|Delay 1e+01 :!label _label)
  (Utilities|IsValid self
    (:Is%20Valid
      (Development|ExecuteConsoleCommand "pv.KillfeedEnabled 0" 0)
      (bind _playerstatus (Class|PavlovProxyStatics|GetPavlovPlayerStatus (Variables|/Script/Engine.Pawn|GetPlayerState (Class|PavlovPlayerProxy|GetPawn))))
      (Development|PrintString (Utilities|String|Append "Player Name:  " (Variables|/Script/Engine.PlayerState|GetPlayerName (.playerstate _playerstatus))) true true "(R=0.082252,G=1.000000,B=0.000000,A=1.000000)" 3e+01)
      (bind _asadmin_game_logic (Utilities|Casting|CastToAdmin_GameLogic (Class|PavlovLibrary|GetGameLogic)))
      (if (or (Utilities|Array|ContainsItem (Variables|/Game/CustomMaps/AdminMenu/Envy/Blueprints/Admin_GameLogic.Admin_GameLogic_C|GetMod%20List _asadmin_game_logic) (Variables|/Script/Engine.PlayerState|GetPlayerName (.playerstate _playerstatus))) (Utilities|Array|ContainsItem (Variables|/Game/CustomMaps/AdminMenu/Envy/Blueprints/Admin_GameLogic.Admin_GameLogic_C|GetMod%20List _asadmin_game_logic) (Variables|Debugging|GetChange%20To%20Mapmaker%20Name%20For%20Debugging)))
        (Class|PavlovPlayerProxy|SetPlayerSkin "Admin")
        (Variables|/Script/Engine.Actor|SetbCanBeDamaged (Class|PavlovPlayerProxy|GetPawn) false)
        (CallFunction|SpawnMyAdminServer)
        (else
          (Class|PavlovPlayerProxy|SetPlayerSkin "StarWars")
          (CallFunction|SpawnMyAdminServer))))
    (:Is%20Not%20Valid
      (goto _label))))

(fn ConstructionScript)

(fn SetMenuandLocktoHand
  (params (WidgetClass :type Actor%20Class%20Reference))
  (bind _returnvalue (Class|PavlovPlayerProxy|GetPawn))
  (bind _handsproxy (Variables|Default|GetHandsProxy))
  (bind _returnvalue_2 (Transformation|GetAttachParent (.nondominanthand _handsproxy)))
  (bind _returnvalue_3 (Transformation|GetAttachParent (.dominanthand _handsproxy)))
  (bind _returnvalue_4 (Transformation|GetAttachParent _returnvalue_2))
  (bind _returnvalue_5 (Transformation|GetAttachParent _returnvalue_3))
  (bind _returnvalue_6 (Transformation|GetAttachParent _returnvalue_4))
  (bind _returnvalue_7 (Transformation|GetAttachParent _returnvalue_5))
  (CallFunction|ServerMarkDominant)
  (bind _returnvalue_8 (Game|SpawnActorfromClass WidgetClass (Transformation|GetWorldTransform _returnvalue_6) "Undefined" _returnvalue 0))
  (bind _output_get (Variables|Gameplay|SetAdminMenuRef _returnvalue_8))
  (Transformation|AttachComponentToComponent _output_get _returnvalue_6 "None" "SnapToTarget" "SnapToTarget" "KeepWorld" true)
  (bind _returnvalue_9 (Game|SpawnActorfromClass "/Game/CustomMaps/AdminMenu/Envy/AdminMenu/WidgetInteractor.WidgetInteractor_C" (Transformation|GetWorldTransform _returnvalue_7) "Undefined" _returnvalue 0))
  (bind _output_get_2 (Variables|Gameplay|SetWidgetInteractor _returnvalue_9))
  (Transformation|AttachComponentToComponent _output_get_2 _returnvalue_7 "None" "SnapToTarget" "SnapToTarget" "KeepWorld" true))