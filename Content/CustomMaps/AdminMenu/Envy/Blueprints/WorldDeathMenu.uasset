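; WorldDeathMenu is an admin menu actor that carries a Widget component, shown on demand by the scoreboard inputs.
; Pressing either ScoreboardLeft or ScoreboardRight makes the widget visible and releasing either hides it, without propagating to child components.
; Tick destroys the actor once its owner is no longer valid.
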(event EventTick
  (params (DeltaSeconds :type Float%20%28single-precision%29))
  (Utilities|IsValid (Components|GetOwner)
    (:Is%20Not%20Valid
      (Actor|DestroyActor))))

(event Input|ActionEvents|InputActionScoreboardLeft
  (params (Key :type Key%20Structure))
  (bind _widget (Variables|Default|GetWidget))
  (:Pressed
    (Rendering|SetVisibility _widget true false))
  (:Released
    (Rendering|SetVisibility _widget false false)))

(event Input|ActionEvents|InputActionScoreboardRight
  (params (Key :type Key%20Structure))
  (bind _widget (Variables|Default|GetWidget))
  (:Pressed
    (Rendering|SetVisibility _widget true false))
  (:Released
    (Rendering|SetVisibility _widget false false)))

(fn ConstructionScript)