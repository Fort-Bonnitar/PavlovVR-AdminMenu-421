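; Pavlov game-mode logic for the AdminMenu custom map, with fall damage disabled and menu-driven item and vehicle spawning for named players.
; Round states start a looping respawn timer, spawn pawns, build the moderator list and end the match.
; Player spawns trigger the spawn UI through Admin_PlayerProxy, and CheckPlayer gives listed moderators an inventory item.
; Helper functions cover respawning, alive counts, killing, scoring and random player selection.
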(event Custom|StartRespawnLoop
  ;[1 1 1] Respawn Loop
  (bind _returnvalue (Utilities|Time|SetTimerbyEvent (EventDispatchers|CreateEvent :!event RespawnLoopBody) 1.0 true))
  (Variables|Respawn|SetRespawnLoop_Handle _returnvalue))

(event Custom|SpawnItemFromMenu
  (params (Id :type Name) (Player%20Name :type String))
  ;[1 1 1] Spawn WEapons Admin
  (for _array_element (select (Variables|GameModeSettings|GetDebug%20Build) (Helpers|GetPlayers) (Variables|Core|GetCurrent%20Players))
    (if (Utilities|Enum|Equal(Enum) (Variables|/Script/Engine.PlayerState|GetPlayerName _array_element) Player%20Name)
      (Class|PavlovGameLogic|SpawnItem (Utilities|Struct|MakePavlovItemSpawnParams :Id Id :Player _array_element :bSpawnWithMagazine true)))))

(event Custom|Spawn%20Player
  (params (Pawn :type Pawn%20Object%20Reference))
  ;[1 1 1] SPawn Player Custom
  (bind _asadmin_player_proxy (Utilities|Casting|CastToAdmin_PlayerProxy (Class|PavlovLibrary|GetPlayerProxy Pawn)))
  (Default|TriggerSpawnUI _asadmin_player_proxy))

(event Custom|SpawnVehicleFromMenu
  (params (VehicleID :type Name) (Player%20Name :type String))
  ;[1 1 1] SpawnVehicles Admin
  (for _array_element (select (Variables|GameModeSettings|GetDebug%20Build) (Helpers|GetPlayers) (Variables|Core|GetCurrent%20Players))
    (if (Utilities|Enum|Equal(Enum) (Variables|/Script/Engine.PlayerState|GetPlayerName _array_element) Player%20Name)
      (bind _playerstatus (Class|PavlovProxyStatics|GetPavlovPlayerStatus _array_element))
      (bind _transform (Class|PavlovGameLogic|GetSpawnTransform (.controller _playerstatus)))
      (Class|PavlovGameLogic|SpawnVehicleAsync (EventDispatchers|CreateEvent :!event Custom|OnSpawnComplete) VehicleID _transform -1 3e+02))))

(event Custom|OnSpawnComplete
  (params (bSuccessful :type Boolean) (SpawnedActor :type Actor%20Object%20Reference) (ID :type Name))
  ;[1 1 1] SpawnVehicles Admin
  (Variables|Default|SetSpawned%20Vehicle SpawnedActor))

(event EventBeginPlay
  (Class|PavlovGameLogic|SetFallDamage false))

(event EventOnRoundStateChanged
  (params (OldState :type EPavlovRoundState%20Enum :default "Starting") (NewState :type EPavlovRoundState%20Enum :default "Starting"))
  ;[1 1 1] Gme Setup
  (switch Utilities|FlowControl|Switch|SwitchonEPavlovRoundState NewState
    (:Starting
      (CallFunction|StartRespawnLoop))
    (:StandBy
      (Utilities|FlowControl|Delay 2.0)
      (Class|PavlovGameLogic|SpawnandPosessPawns)
      (for _array_element (Variables|Core|GetCurrent%20Players)
        (bind _playerstatus (Class|PavlovProxyStatics|GetPavlovPlayerStatus _array_element))
        (CallFunction|SpawnPlayer (.pawn _playerstatus))))
    (:Started
      (CallFunction|GameSetup)
      (Class|PavlovGameLogic|SetFallDamage false))
    (:Ended
      (Utilities|FlowControl|Delay 5.0)
      (bind _asgame_mode (Utilities|Casting|CastToGameMode (Game|GetGameMode)))
      (Class|GameMode|EndMatch _asgame_mode))))

(event EventOnPlayerSpawned
  (params (PlayerStatus :type Pavlov%20Player%20Status%20Structure%20%28by%20ref%29))
  ;[1 1 1] Spawn Player
  (switch Utilities|FlowControl|Switch|SwitchonEPavlovRoundState (Class|PavlovGameLogic|GetRoundState)
    (:Starting
      (CallFunction|SpawnPlayer (.pawn PlayerStatus)))))

(fn ConstructionScript)

(fn RespawnPlayers
  (params (CheckRespawnTime :type Boolean) (OnlyTeam :type Boolean) (TeamID :type Integer))
  (for _array_element (Helpers|GetPlayers)
    (bind (_playerstatus _bsucceeded) (Class|PavlovProxyStatics|GetPavlovPlayerStatus _array_element))
    (if _bsucceeded
      (if (select OnlyTeam (and (select CheckRespawnTime (and (.bDead (Utilities|Struct|BreakPavlovPlayerStatus _playerstatus)) (>= (.DeadTime (Utilities|Struct|BreakPavlovPlayerStatus _playerstatus)) (Variables|GameLogicSettings|GetRespawnTime))) (.bDead (Utilities|Struct|BreakPavlovPlayerStatus _playerstatus))) (== (.TeamId (Utilities|Struct|BreakPavlovPlayerStatus _playerstatus)) TeamID)) (select CheckRespawnTime (and (.bDead (Utilities|Struct|BreakPavlovPlayerStatus _playerstatus)) (>= (.DeadTime (Utilities|Struct|BreakPavlovPlayerStatus _playerstatus)) (Variables|GameLogicSettings|GetRespawnTime))) (.bDead (Utilities|Struct|BreakPavlovPlayerStatus _playerstatus))))
        (bind _transform (Class|PavlovGameLogic|GetSpawnTransform (.Controller (Utilities|Struct|BreakPavlovPlayerStatus _playerstatus))))
        (Class|PavlovGameLogic|Spawn (.Controller (Utilities|Struct|BreakPavlovPlayerStatus _playerstatus)) _transform false))))
  (return))

(fn GetPlayers
  (return (Variables|/Script/Engine.GameStateBase|GetPlayerArray (Game|GetGameState))))

(fn GetAliveCount
  (params (OnlyTeam :type Boolean) (TeamId :type Integer))
  (for _array_element (Helpers|GetPlayers)
    (bind (_playerstatus _bsucceeded) (Class|PavlovProxyStatics|GetPavlovPlayerStatus _array_element))
    (if _bsucceeded
      (if (select OnlyTeam (and (not (.bDead (Utilities|Struct|BreakPavlovPlayerStatus _playerstatus))) (== (.TeamId (Utilities|Struct|BreakPavlovPlayerStatus _playerstatus)) TeamId)) (not (.bDead (Utilities|Struct|BreakPavlovPlayerStatus _playerstatus))))
        (Math|Integer|IncrementInt (LocalVariables|GetL_AliveCount)))))
  (return (LocalVariables|GetL_AliveCount)))

(fn RespawnPlayer
  (params (PlayerState :type Player%20State%20Object%20Reference) (CheckRespawnTime :type Boolean))
  (Utilities|IsValid PlayerState
    (:Is%20Valid
      (bind (_playerstatus _bsucceeded) (Class|PavlovProxyStatics|GetPavlovPlayerStatus PlayerState))
      (if _bsucceeded
        (if (select CheckRespawnTime (and (.bDead (Utilities|Struct|BreakPavlovPlayerStatus _playerstatus)) (>= (.DeadTime (Utilities|Struct|BreakPavlovPlayerStatus _playerstatus)) (Variables|GameLogicSettings|GetRespawnTime))) (.bDead (Utilities|Struct|BreakPavlovPlayerStatus _playerstatus)))
          (bind _transform (Class|PavlovGameLogic|GetSpawnTransform (.Controller (Utilities|Struct|BreakPavlovPlayerStatus _playerstatus))))
          (Class|PavlovGameLogic|Spawn (.Controller (Utilities|Struct|BreakPavlovPlayerStatus _playerstatus)) _transform false))))
    (:Is%20Not%20Valid
      (return false))))

(fn RespawnLoopBody
  (for _array_element (Helpers|GetPlayers)
    (bind (_playerstatus _bsucceeded) (Class|PavlovProxyStatics|GetPavlovPlayerStatus _array_element))
    (if _bsucceeded
      (if (and (.bDead (Utilities|Struct|BreakPavlovPlayerStatus _playerstatus)) (>= (.DeadTime (Utilities|Struct|BreakPavlovPlayerStatus _playerstatus)) (Variables|GameLogicSettings|GetRespawnTime)))
        (bind _transform (Class|PavlovGameLogic|GetSpawnTransform (.Controller (Utilities|Struct|BreakPavlovPlayerStatus _playerstatus))))
        (Class|PavlovGameLogic|Spawn (.Controller (Utilities|Struct|BreakPavlovPlayerStatus _playerstatus)) _transform false))))
  (return))

(fn StopRespawnLoop
  (Utilities|Time|ClearandInvalidateTimerbyHandle (Variables|Respawn|GetRespawnLoop_Handle))
  (return))

(fn PlayerSpawned
  (params (PlayerStatus :type Pavlov%20Player%20Status%20Structure%20%28by%20ref%29))
  ;[1 1 1] This return does nothing, it just prevents the function from creating an event in the graph if you override it
  (return false))

(fn PlayerKilled
  (params (PlayerStatus :type Pavlov%20Player%20Status%20Structure%20%28by%20ref%29) (Killer :type Player%20State%20Object%20Reference) (bHeadshot :type Boolean) (KilledByItem :type Name))
  ;[1 1 1] This return does nothing, it just prevents the function from creating an event in the graph if you override it
  (return false))

(fn EnoughPlayerstoStart
  (params (PlayerCountToStart :type Integer))
  (return (>= (Utilities|Array|Length (Helpers|GetPlayers)) PlayerCountToStart)))

(fn IsRoundState?
  (params (RoundState :type EPavlovRoundState%20Enum :default "Starting"))
  (return (Utilities|Enum|Equal(Enum) (Class|PavlovGameLogic|GetRoundState) RoundState)))

(fn KillAllAlivePlayers
  (for _array_element (Helpers|GetPlayers)
    (bind (_playerstatus _bsucceeded) (Class|PavlovProxyStatics|GetPavlovPlayerStatus _array_element))
    (if _bsucceeded
      (if (and (Utilities|IsValid (.Pawn (Utilities|Struct|BreakPavlovPlayerStatus _playerstatus))) (not (.bDead (Utilities|Struct|BreakPavlovPlayerStatus _playerstatus))))
        (Game|Damage|ApplyDamage (.Pawn (Utilities|Struct|BreakPavlovPlayerStatus _playerstatus)) 99999.0 0 0))))
  (return))

(fn WasRevived?
  (params (PlayerState :type Player%20State%20Object%20Reference))
  (Utilities|IsValid PlayerState
    (:Is%20Valid
      (if (Actor|ActorHasTag PlayerState "Revived")
        (Utilities|Array|RemoveItem (Variables|/Script/Engine.Actor|GetTags PlayerState) "Revived")
        (return true)
        (else
          _)))
    (:Is%20Not%20Valid
      _))
  (return false))

(fn GetRandomPlayer
  (params (Player%20List :type Array%20of%20Player%20State%20Object%20References) (%20Ignore :type Array%20of%20Player%20State%20Object%20References))
  (bind _returnvalue (Math|DateTime|Now))
  (LocalVariables|SetPlayers Player%20List)
  (for _array_element %20Ignore
    (Utilities|IsValid _array_element
      (:Is%20Valid
        (Utilities|Array|RemoveItem (LocalVariables|GetPlayers) _array_element))))
  (Utilities|Array|Shuffle (LocalVariables|GetPlayers))
  (bind _output_get (LocalVariables|SetRandom%20Player (Utilities|Array|Get(acopy) (LocalVariables|GetPlayers) (Math|Random|RandomIntegerinRangefromStream 0 (- (Utilities|Array|Length (LocalVariables|GetPlayers)) 1) (Math|Random|MakeRandomStream (* (+ (.year _returnvalue) 1) (+ (.month _returnvalue) 1) (+ (.day _returnvalue) 1) (+ (.hour _returnvalue) 1) (+ (.minute _returnvalue) 1) (+ (.second _returnvalue) 1) (+ (.millisecond _returnvalue) 1)))))))
  (return _output_get))

(fn SetPlayerScore
  (params (Player%20State :type Player%20State%20Object%20Reference) (Score :type Integer))
  (bind _playerstatus (Class|PavlovProxyStatics|GetPavlovPlayerStatus Player%20State))
  (Class|PavlovGameLogic|IncrementPlayerScore (.playerstate _playerstatus) (- Score (.score _playerstatus)))
  (return))

(fn CheckAlivePlayers
  (LocalVariables|SetAC 0)
  (for _array_element (select (Variables|GameModeSettings|GetDebug%20Build) (Helpers|GetPlayers) (Variables|Core|GetCurrent%20Players))
    (Utilities|IsValid _array_element
      (:Is%20Valid
        (if (and (not (Actor|ActorHasTag _array_element "DeadEmployee")) (not (Actor|ActorHasTag _array_element "Murderer")))
          (Math|Integer|IncrementInt (LocalVariables|GetAC))))))
  (return (LocalVariables|GetAC)))

(fn GameSetup
  (bind (_bsuccessful _mods) (Class|PavlovLibrary|GetModerators))
  (if _bsuccessful
    (Variables|Moderation|SetMod%20List _mods)
    (Utilities|Array|AddUnique (Variables|Moderation|GetMod%20List) (Variables|Default|GetMapMakerNameForDebugging))
    (else
      (Variables|Moderation|SetMod%20List (Utilities|Array|MakeArray (Variables|Default|GetMapMakerNameForDebugging))))))

(fn CheckPlayer
  (params (PlayerState :type Player%20State%20Object%20Reference))
  (if (Utilities|Array|ContainsItem (Variables|Moderation|GetMod%20List) (Variables|/Script/Engine.PlayerState|GetPlayerName PlayerState))
    (Class|PavlovGameLogic|SpawnItem (Utilities|Struct|MakePavlovItemSpawnParams "ID" PlayerState false true 7 false "" false false))
    (return true)
    (else
      (return false))))